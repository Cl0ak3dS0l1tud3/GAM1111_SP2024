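; Door actor Blueprint that raises a door mesh on the RaiseDoor event (commented as a button press) and lowers it again.
; A RaiseDoor timeline sets the door's relative location through VectorSlerpNormals between fixed zero and raised vectors.
; Any actor leaving DoorCollision reverses the timeline, as the player check is unconnected.
; BeginPlay caches start and end locations, which the animation never reads.
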(event OnComponentEndOverlap(DoorCollision)
  (params (OverlappedComponent :type Primitive%20Component%20Object%20Reference) (OtherActor :type Actor%20Object%20Reference) (OtherComp :type Primitive%20Component%20Object%20Reference) (OtherBodyIndex :type Integer))
  ;[1 1 1] Door Lowers Once Player Leaves Collision
  ;[1 1 1] Door Raises When Button Is Pressed
  (bind _raise_door (Timeline|Raise%20Door Reverse)
    (:Update
      (Transformation|SetRelativeLocation (Variables|Default|GetMyDoor) (Class|KismetMathLibrary|VectorSlerpNormals "0, 0, 0" "0.000000,0.000000,200.000000" _raise_door) false false))))

(event EventBeginPlay
  (bind _mydoor (Variables|Default|GetMyDoor))
  (bind _relativelocation (Variables|/Script/Engine.SceneComponent|GetRelativeLocation _mydoor))
  (bind (_x _y _z) (Math|Vector|BreakVector _relativelocation))
  ;[1 1 1] Fetches Door's Location To Play Animation
  (Utilities|FlowControl|Sequence
    (:then_0
      (Variables|Default|SetRaiseDoorLocBeg _relativelocation)
      (Variables|Default|SetRaiseDoorLocEnd (Math|Vector|MakeVector _x _y (+ _z 2e+02))))
    (:then_1
      (Components|Timeline|SetPlayRate (Variables|Default|GetRaise%20Door) 1.0))))

(event EventTick
  (params (DeltaSeconds :type Float%20%28single-precision%29)))

(event EventRaiseDoor
  ;[1 1 1] Door Raises When Button Is Pressed
  (bind _raise_door (Timeline|Raise%20Door Play)
    (:Update
      (Transformation|SetRelativeLocation (Variables|Default|GetMyDoor) (Class|KismetMathLibrary|VectorSlerpNormals "0, 0, 0" "0.000000,0.000000,200.000000" _raise_door) false false))))

(event Collision|EventActorBeginOverlap
  (params (OtherActor :type Actor%20Object%20Reference)))

(fn ConstructionScript)