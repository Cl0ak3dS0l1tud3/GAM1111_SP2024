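; Interactive button actor that rises when approached and, when pressed, signals its linked door to open.
; Any actor overlapping ButtonCollision plays the ButtonUp timeline, which raises the button and enables player input on finish; leaving reverses it.
; Interact plays the ButtonPress timeline between positions cached at BeginPlay, using a normal slerp.
; When the forward press finishes, it reverses and calls RaiseDoorMessage on MyDoor.
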(event OnComponentBeginOverlap(ButtonCollision)
  (params (OverlappedComponent :type Primitive%20Component%20Object%20Reference) (OtherActor :type Actor%20Object%20Reference) (OtherComp :type Primitive%20Component%20Object%20Reference) (OtherBodyIndex :type Integer) (bFromSweep :type Boolean) (SweepResult :type Hit%20Result%20Structure%20%28by%20ref%29))
  ;[1 1 1] Button Goes Up On Collision (or down when player leaves)
  (if true
    (bind _buttonraise (Timeline|ButtonUp Play)
      (:Update
        (Transformation|SetRelativeLocation (Variables|Default|GetButtonPress) (Math|Vector|Lerp(Vector) "0.000000,0.000000,53.000000" "0.000000,0.000000,72.000000" _buttonraise) false false))
      (:Finished
        (Input|EnableInput (Game|GetPlayerController 0))))))

(event OnComponentEndOverlap(ButtonCollision)
  (params (OverlappedComponent :type Primitive%20Component%20Object%20Reference) (OtherActor :type Actor%20Object%20Reference) (OtherComp :type Primitive%20Component%20Object%20Reference) (OtherBodyIndex :type Integer))
  ;[1 1 1] Button Goes Up On Collision (or down when player leaves)
  (if true
    (bind _buttonraise (Timeline|ButtonUp Reverse)
      (:Update
        (Transformation|SetRelativeLocation (Variables|Default|GetButtonPress) (Math|Vector|Lerp(Vector) "0.000000,0.000000,53.000000" "0.000000,0.000000,72.000000" _buttonraise) false false))
      (:Finished
        (Input|EnableInput (Game|GetPlayerController 0))))))

(event Input|EnhancedActionEvents|EnhancedInputActionInteract
  (params (ActionValue :type Boolean) (ElapsedSeconds :type Float%20%28double-precision%29) (TriggeredSeconds :type Float%20%28double-precision%29) (InputAction :type Input%20Action%20Object%20Reference :default "/Game/ThirdPerson/Input/Actions/Interact.Interact"))
  ;[1 1 1] Pressing "E" Pushes Button Down and Tells Door To Open
  (bind (_direction _buttonpressgoesdown) (Timeline|Button%20Press Play)
    (:Update
      (Transformation|SetRelativeLocation (Variables|Default|GetButtonPress) (Class|KismetMathLibrary|VectorSlerpNormals (Variables|Default|GetButtonPressLocBeg) (Variables|Default|GetButtonPressLocEnd) _buttonpressgoesdown) false false))
    (:Finished
      (switch Utilities|FlowControl|Switch|SwitchonETimelineDirection _direction
        (:Forward
          (Utilities|FlowControl|Sequence
            (:then_0
              (Timeline|Button%20Press Reverse))
            (:then_1
              (Class|PinnelloDoorProjectINT|RaiseDoor(Message) (Variables|Default|GetMyDoor)))))))))

(event EventBeginPlay
  (bind _buttonpress (Variables|Default|GetButtonPress))
  (bind _relativelocation (Variables|/Script/Engine.SceneComponent|GetRelativeLocation _buttonpress))
  (bind (_x _y _z) (Math|Vector|BreakVector _relativelocation))
  ;[1 1 1] Fetches The Button's Current Location For The Animation
  (Utilities|FlowControl|Sequence
    (:then_0
      (Variables|Default|SetButtonPressLocBeg _relativelocation)
      (Variables|Default|SetButtonPressLocEnd (Math|Vector|MakeVector _x _y (+ _z 19.0))))
    (:then_1
      (Components|Timeline|SetPlayRate (Variables|Default|GetButton%20Press) 0.0))))

(event EventTick
  (params (DeltaSeconds :type Float%20%28single-precision%29)))

(event Collision|EventActorBeginOverlap
  (params (OtherActor :type Actor%20Object%20Reference)))

(fn ConstructionScript)